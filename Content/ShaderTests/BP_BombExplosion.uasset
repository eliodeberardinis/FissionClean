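; BP_BombExplosion is a bomb explosion actor that combines a particle effect, a radial force impulse and explosion audio.
; On BeginPlay it enables input from player controller 0, so pressing Q activates the particles, fires the impulse and plays the sound after a short delay.
; A separate ExplodeBase function runs the same sequence without the delay and is not called within this Blueprint.
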(event EventBeginPlay
  (Input|EnableInput (Game|GetPlayerController 0)))

(event Input|KeyboardEvents|Q
  (params (Key :type Key%20Structure :default "AnyKey"))
  (:Pressed
    (Components|Activation|Activate (Variables|Default|GetP_Explosion) false)
    (Class|RadialForceComponent|FireImpulse (Variables|Default|GetBomb_RadialForce))
    (Utilities|FlowControl|Delay 0.2)
    (Audio|Components|Audio|Play (Variables|Default|GetExplosion%20Audio) 0.0)))

(fn ConstructionScript)

(fn ExplodeBase
  (Components|Activation|Activate (Variables|Default|GetP_Explosion) false)
  (Class|RadialForceComponent|FireImpulse (Variables|Default|GetBomb_RadialForce))
  (Audio|Components|Audio|Play (Variables|Default|GetExplosion%20Audio) 0.0))