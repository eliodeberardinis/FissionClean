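; Global climate controller that toggles the world between winter and non-winter looks, with a rust toggle alongside.
; ChangeWeather, triggered by a temporary E key or ToggleWeatherSystem, plays or reverses timelines writing rust, moss/snow, ground snow and frost scalars to MPC_GlobalSeasonCycle.
; It also toggles a snow emitter, repositioned over the player only on each toggle.
; Frosted-lens post-processing is disabled once its reverse fade finishes.
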(event Custom|ChangeWeather
  (bind _p_snow (Variables|Default|GetP_Snow))
  (bind _player (Variables|Default|GetPlayer))
  (bind _postprocessfrost (Variables|Default|GetPostProcessFrost))
  (bind _returnvalue (Transformation|GetActorLocation _player))
  (Utilities|FlowControl|Sequence
    (:then_0
      ;[1 1 1] Rust
      (if (Variables|Default|GetisRusted)
        (Variables|Default|SetisRusted false)
        (bind (_direction _bn _op _wbm) (Timeline|Timeline_0 Reverse)
          (:Update
            (Rendering|Material|SetScalarParameterValue "/Game/ShaderTests/MPC_GlobalSeasonCycle.MPC_GlobalSeasonCycle" "R_BlendNormal" _bn :!class /Script/Engine.KismetMaterialLibrary)
            (Rendering|Material|SetScalarParameterValue "/Game/ShaderTests/MPC_GlobalSeasonCycle.MPC_GlobalSeasonCycle" "R_Opacity" _op :!class /Script/Engine.KismetMaterialLibrary)
            (Rendering|Material|SetScalarParameterValue "/Game/ShaderTests/MPC_GlobalSeasonCycle.MPC_GlobalSeasonCycle" "R_WorldBlendMax" _wbm :!class /Script/Engine.KismetMaterialLibrary)))
        (else
          (Variables|Default|SetisRusted true)
          (Timeline|Timeline_0 Play))))
    (:then_1
      ;[1 1 1] Moss and Snow
      (if (Variables|Default|GetisWinter)
        (bind (_direction_2 _mossvsnow_value _opacity_value _roughness_value _blendnormal _worldblendmax) (Timeline|MossAndSnowTimer Reverse)
          (:Update
            (Rendering|Material|SetScalarParameterValue "/Game/ShaderTests/MPC_GlobalSeasonCycle.MPC_GlobalSeasonCycle" "MS_MossVSnow" _mossvsnow_value :!class /Script/Engine.KismetMaterialLibrary)
            (Rendering|Material|SetScalarParameterValue "/Game/ShaderTests/MPC_GlobalSeasonCycle.MPC_GlobalSeasonCycle" "MS_Opacity" _opacity_value :!class /Script/Engine.KismetMaterialLibrary)
            (Rendering|Material|SetScalarParameterValue "/Game/ShaderTests/MPC_GlobalSeasonCycle.MPC_GlobalSeasonCycle" "MS_Roughness" _roughness_value :!class /Script/Engine.KismetMaterialLibrary)
            (Rendering|Material|SetScalarParameterValue "/Game/ShaderTests/MPC_GlobalSeasonCycle.MPC_GlobalSeasonCycle" "MS_BlendNormal" _blendnormal :!class /Script/Engine.KismetMaterialLibrary)
            (Rendering|Material|SetScalarParameterValue "/Game/ShaderTests/MPC_GlobalSeasonCycle.MPC_GlobalSeasonCycle" "MS_WorldBlendMax" _worldblendmax :!class /Script/Engine.KismetMaterialLibrary)))
        (else
          (Timeline|MossAndSnowTimer Play))))
    (:then_2
      ;[1 1 1] Particle Snow System AND Ground Snow
      (if (Variables|Default|GetisWinter)
        (Components|Activation|Deactivate _p_snow)
        (bind (_direction_3 _groundbn _groundo _groundwbm) (Timeline|SnowParticleSystemTimer Reverse)
          (:Update
            (Rendering|Material|SetScalarParameterValue "/Game/ShaderTests/MPC_GlobalSeasonCycle.MPC_GlobalSeasonCycle" "GS_BlendNormal" _groundbn :!class /Script/Engine.KismetMaterialLibrary)
            (Rendering|Material|SetScalarParameterValue "/Game/ShaderTests/MPC_GlobalSeasonCycle.MPC_GlobalSeasonCycle" "GS_Opacity" _groundo :!class /Script/Engine.KismetMaterialLibrary)
            (Rendering|Material|SetScalarParameterValue "/Game/ShaderTests/MPC_GlobalSeasonCycle.MPC_GlobalSeasonCycle" "GS_WorldBlendMax" _groundwbm :!class /Script/Engine.KismetMaterialLibrary)))
        (else
          (Components|Activation|Activate _p_snow false)
          (Timeline|SnowParticleSystemTimer Play))))
    (:then_3
      ;[1 1 1] Frosted Lens PostProcessing Effect
      (if (Variables|Default|GetisWinter)
        (Variables|Default|SetisWinter false)
        (Variables|Default|SetdestroyFrost true)
        (bind (_direction_4 _frostdensity _frostopacity) (Timeline|FrostPPCycle Reverse)
          (:Update
            ;;[1 1 1] Fade in from edges
            (Rendering|Material|SetScalarParameterValue "/Game/ShaderTests/MPC_GlobalSeasonCycle.MPC_GlobalSeasonCycle" "F_Density" _frostdensity :!class /Script/Engine.KismetMaterialLibrary)
            (Rendering|Material|SetScalarParameterValue "/Game/ShaderTests/MPC_GlobalSeasonCycle.MPC_GlobalSeasonCycle" "F_Opacity" _frostopacity :!class /Script/Engine.KismetMaterialLibrary))
          (:Finished
            ;;[1 1 1] Disable PP after anim
            (if (Variables|Default|GetdestroyFrost)
              (Variables|/Script/Engine.PostProcessComponent|SetbEnabled _postprocessfrost false)
              (Variables|Default|SetdestroyFrost false))))
        (else
          (Variables|Default|SetisWinter true)
          (Variables|/Script/Engine.PostProcessComponent|SetbEnabled _postprocessfrost true)
          (Variables|Default|SetdestroyFrost false)
          (Timeline|FrostPPCycle Play))))
    (:then_4
      ;[1 1 1] Set Snow Location
      (Transformation|SetWorldLocation (Variables|Default|GetP_Snow) (Math|Vector|MakeVector (.x _returnvalue) (.y _returnvalue) 1.01e+03) false false))))

(event EventBeginPlay
  (bind _returnvalue (Game|GetPlayerController 0))
  (bind _returnvalue_2 (Transformation|GetActorLocation _returnvalue))
  ;[1 1 1] Enable INput
  (Input|EnableInput (Game|GetPlayerController 0))
  ;[1 1 1] Init Particle Snow Emitter
  (bind _returnvalue_3 (Effects|SpawnEmitteratLocation "/Game/ShaderTests/P_Snow.P_Snow" (Math|Vector|MakeVector (.x _returnvalue_2) (.y _returnvalue_2) 1.01e+03) "0, 0, 0" false))
  (Variables|Default|SetP_Snow _returnvalue_3)
  (Components|Activation|Deactivate (Variables|Default|GetP_Snow))
  ;[1 1 1] Default Frost Post Processing to disabled
  (Variables|/Script/Engine.PostProcessComponent|SetbEnabled (Variables|Default|GetPostProcessFrost) false)
  (Variables|Default|SetisWinter false)
  ;[1 1 1] Get Player reference for snow particle location
  (bind _outactors (Actor|GetAllActorsOfClass "/Game/ThirdPersonBP/Blueprints/ThirdPersonCharacter.ThirdPersonCharacter_C"))
  (Variables|Default|SetPlayer (Utilities|Array|Get(acopy) _outactors)))

(event Input|KeyboardEvents|E
  (params (Key :type Key%20Structure :default "AnyKey"))
  ;[1 1 1] TMP
  (:Pressed
    (CallFunction|ChangeWeather)))

(fn ConstructionScript)

(fn ToggleWeatherSystem
  (CallFunction|ChangeWeather))