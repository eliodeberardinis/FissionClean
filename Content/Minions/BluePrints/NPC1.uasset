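; NPC1 is a minion character that follows the player on perception updates and returns to its starting post when it stops.
; BeginPlay caches the player and its own starting transform.
; Each perception update flips a Watch/Follow state: Follow repeats AI MoveTo toward the player while the stimulus reads as sensed.
; Watch halts movement, waits briefly, then walks home and restores the original rotation if still watching.
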(event OnTargetPerceptionUpdated(AIPerception)
  (params (Actor :type Actor%20Object%20Reference) (Stimulus :type AI%20Stimulus%20Structure))
  (switch Utilities|FlowControl|Switch|SwitchonStates_NPC1 (Variables|Default|GetStates)
    (:NewEnumerator0
      (Variables|Default|SetStates "NewEnumerator1")
      (AI|AIMoveTo self "0, 0, 0" (Variables|Default|GetPlayer) 1.5e+02 false :!label _label
        (:OnSuccess
          (if (.bSuccessfullySensed (Utilities|Struct|BreakAIStimulus Stimulus))
            (goto _label)))))
    (:NewEnumerator1
      (Variables|Default|SetStates "NewEnumerator0")
      (Components|Movement|StopMovementImmediately (Variables|Character|GetCharacterMovement))
      (Utilities|FlowControl|Delay 2.0)
      (if (Utilities|Enum|Equal(Enum) (Variables|Default|GetStates) "NewEnumerator0")
        (AI|AIMoveTo self (Variables|Default|GetInitialLocation) 0 5.0 false
          (:OnSuccess
            (Transformation|SetActorRotation (Variables|Default|GetInitialRotation))))))))

(event EventBeginPlay
  (bind _asthird_person_character (Utilities|Casting|CastToThirdPersonCharacter (Game|GetPlayerCharacter 0)))
  (Variables|Default|SetPlayer _asthird_person_character)
  (Variables|Default|SetInitialLocation (Transformation|GetActorLocation))
  (Variables|Default|SetInitialRotation (Transformation|GetActorRotation)))

(fn ConstructionScript)