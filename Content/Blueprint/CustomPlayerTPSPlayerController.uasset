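; Third-person shooter player controller Blueprint that supplies view location and aim direction queries.
; ViewPoint returns the follow camera's view location on a possessed ThirdPersonCharacter, falling back to the controller's focal location otherwise.
; AimVector returns the forward vector of the controlled pawn's base aim rotation, or of the control rotation when no valid pawn exists.
; The event graph and construction script contain no logic.
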(event EventBeginPlay)

(event EventTick
  (params (DeltaSeconds :type Float%20%28single-precision%29)))

(fn ConstructionScript)

(fn ViewPoint
  (Variables|Default|SetOutViewLocation "0, 0, 0")
  (bind _asthird_person_character (Utilities|Casting|CastToThirdPersonCharacter (Pawn|GetControlledPawn))
    (:then
      (bind _desiredview (Class|CameraComponent|GetCameraView (Variables|/Game/ThirdPersonBP/Blueprints/ThirdPersonCharacter.ThirdPersonCharacter_C|GetFollowCamera _asthird_person_character) 0.0))
      (Variables|Default|SetOutViewLocation (.location _desiredview)))
    (:CastFailed
      (Variables|Default|SetOutViewLocation (Class|PlayerController|GetFocalLocation))))
  (return (Variables|Default|GetOutViewLocation)))

(fn AimVector
  (bind _returnvalue (Pawn|GetControlledPawn))
  (Utilities|IsValid _returnvalue
    (:Is%20Valid
      (LocalVariables|SetOutAim (Math|Vector|GetForwardVector (Pawn|GetBaseAimRotation _returnvalue))))
    (:Is%20Not%20Valid
      (LocalVariables|SetOutAim (Math|Rotator|GetRotationXVector (Pawn|GetControlRotation :!class /Script/Engine.Controller)))))
  (return (LocalVariables|GetOutAim)))