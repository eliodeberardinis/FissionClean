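; RagdollRick is a test actor that ragdolls when H is pressed or ApplyRagdoll is called, then destroys itself a second later.
; Both triggers share an authority switch: authority calls UpdateRagdoll directly, while remote goes through ClientUpdateRagsoll, and both reach DoRagdoll.
; DoRagdoll enables physics on the skeletal mesh and applies a strong radial impulse using ApplyRagdoll's vector and object.
; Debug prints mark each path.
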(event Custom|UpdateRagdoll
  (CallFunction|DoRagdoll self))

(event Custom|Client%20Update%20Ragsoll
  (CallFunction|UpdateRagdoll))

(event Custom|DoRagdoll
  (Physics|SetSimulatePhysics (Variables|SkeletalMeshActor|GetSkeletalMeshComponent) true)
  (Physics|AddRadialImpulse (stale Custom|ApplyRagdoll Obj) (stale Custom|ApplyRagdoll Vec) 1e+02 577799.0 "RIF_Constant" false)
  (Development|PrintString "ouch!")
  (Utilities|FlowControl|Delay 1.0)
  (Actor|DestroyActor))

(event Custom|ApplyRagdoll
  (params (Vec :type Vector) (Obj :type Primitive%20Component%20Object%20Reference))
  (Networking|SwitchHasAuthority
    (:Authority
      (Development|PrintString "server")
      (CallFunction|UpdateRagdoll))
    (:Remote
      (Development|PrintString "client")
      (CallFunction|ClientUpdateRagsoll))))

(event EventBeginPlay
  (Input|EnableInput (Game|GetPlayerController 0)))

(event Input|KeyboardEvents|H
  (params (Key :type Key%20Structure :default "AnyKey"))
  (:Pressed
    (Networking|SwitchHasAuthority
      (:Authority
        (Development|PrintString "server")
        (CallFunction|UpdateRagdoll))
      (:Remote
        (Development|PrintString "client")
        (CallFunction|ClientUpdateRagsoll)))))

(fn ConstructionScript)