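; Tug-of-war payload cart that red and blue teams push along a CartSpline_BP track toward the enemy base, against a countdown.
; Trigger overlaps sum tagged player and minion forces into direction and speed; a lone team's player overrides minions.
; Tick moves the cart by spline distance, mapped to signed progress.
; Progress thresholds block the opposing team and reset the timer, toggle speed-changing winter weather, or explode the base to end the game.
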(event OnComponentBeginOverlap(ProximityTrigger)
  (params (OverlappedComponent :type Primitive%20Component%20Object%20Reference) (OtherActor :type Actor%20Object%20Reference) (OtherComp :type Primitive%20Component%20Object%20Reference) (OtherBodyIndex :type Integer) (bFromSweep :type Boolean) (SweepResult :type Hit%20Result%20Structure%20%28by%20ref%29))
  ;[1 1 1] Update Cart Movement and Direction
  ;;[1 1 1] Player or minion of red or blue team enters cart push trigger
  ;;;[1 1 1] Check Trigger for Player Character
  (bind _asthird_person_character (Utilities|Casting|CastToThirdPersonCharacter OtherActor)
    (:then
      (if (and (not (Variables|GameManager|GetRedDidWin)) (not (Variables|GameManager|GetBlueDidWin)))
        ;;;[1 1 1] influence direction based off player team
        ;;; Red = 1
        ;;; Blue = -1
        (if (and (Actor|ActorHasTag _asthird_person_character "PlayerRed") (Variables|GameManager|GetRedCanPush))
          ;;;[1 1 1] Update player is pushing cart
          ;;;;[1 0 0] Red
          (bind _output_get (Variables|CartMovement|SetRedAndBlueForces (+ (Variables|CartMovement|GetRedAndBlueForces) (Variables|CartMovement|GetPlayerCartForce))))
          (Variables|CartMovement|SetRedPlayerIsAtCart true)
          (CallFunction|UpdateCartDirection _output_get)
          ;;;[1 1 1] Set Cart Speed with Direction
          (Variables|CartProgress|SetCartSpeed (* (Variables|CartProgress|GetCurCartVelocity) (Variables|CartProgress|GetCartDirection)) :!label _label)
          (elif (and (Actor|ActorHasTag _asthird_person_character "PlayerBlue") (Variables|GameManager|GetBlueCanPush))
            ;;;;[0 0 1] Blue
            (bind _output_get_2 (Variables|CartMovement|SetRedAndBlueForces (- (Variables|CartMovement|GetRedAndBlueForces) (Variables|CartMovement|GetPlayerCartForce))))
            (Variables|CartMovement|SetBluePlayerIsAtCart true)
            (CallFunction|UpdateCartDirection _output_get_2)
            (goto _label)))))
    (:CastFailed
      ;;;[1 1 1] Check for Minion
      (bind _asminion_test (Utilities|Casting|CastToMinionTest OtherActor))
      ;;;[1 1 1] Else if Minion, increment minion count, if >3 move cart
      (if (and (Actor|ActorHasTag _asminion_test "MinionRed") (Variables|GameManager|GetRedCanPush))
        ;;;;[1 0 0] Red
        (bind _output_get_3 (Variables|CartMovement|SetRedAndBlueForces (+ (Variables|CartMovement|GetRedAndBlueForces) (Variables|CartMovement|GetMinionCartForce))))
        (CallFunction|UpdateCartDirection _output_get_3)
        ;;;[1 1 1] Set Cart Speed with Direction
        (Variables|CartProgress|SetCartSpeed (* (Variables|CartProgress|GetCurCartVelocity) (Variables|CartProgress|GetCartDirection)) :!label _label_2)
        (elif (and (Actor|ActorHasTag _asminion_test "MinionBlue") (Variables|GameManager|GetBlueCanPush))
          ;;;;[0 0 1] Blue
          (bind _output_get_4 (Variables|CartMovement|SetRedAndBlueForces (- (Variables|CartMovement|GetRedAndBlueForces) (Variables|CartMovement|GetMinionCartForce))))
          (CallFunction|UpdateCartDirection _output_get_4)
          (goto _label_2))))))

(event OnComponentEndOverlap(ProximityTrigger)
  (params (OverlappedComponent :type Primitive%20Component%20Object%20Reference) (OtherActor :type Actor%20Object%20Reference) (OtherComp :type Primitive%20Component%20Object%20Reference) (OtherBodyIndex :type Integer))
  ;[1 1 1] Update Cart Movement and Direction
  ;;[1 1 1] Player or minion of either team leaves cart push trigger
  (bind _asthird_person_character (Utilities|Casting|CastToThirdPersonCharacter OtherActor)
    (:then
      (if (and (not (Variables|GameManager|GetRedDidWin)) (not (Variables|GameManager|GetBlueDidWin)))
        ;;;[1 1 1] influence direction based off player team
        ;;; Red = 1
        ;;; Blue = -1
        (if (and (Actor|ActorHasTag _asthird_person_character "PlayerRed") (Variables|GameManager|GetRedCanPush))
          ;;;[1 1 1] Update player is pushing cart
          ;;;;[1 0 0] Red
          (bind _output_get (Variables|CartMovement|SetRedAndBlueForces (- (Variables|CartMovement|GetRedAndBlueForces) (Variables|CartMovement|GetPlayerCartForce))))
          (Variables|CartMovement|SetRedPlayerIsAtCart false)
          (CallFunction|UpdateCartDirection _output_get)
          ;;;[1 1 1] Set Cart Speed with Direction
          (Variables|CartProgress|SetCartSpeed (* (Variables|CartProgress|GetCurCartVelocity) (Variables|CartProgress|GetCartDirection)) :!label _label)
          (elif (and (Actor|ActorHasTag _asthird_person_character "PlayerBlue") (Variables|GameManager|GetBlueCanPush))
            ;;;;[0 0 1] Blue
            (bind _output_get_2 (Variables|CartMovement|SetRedAndBlueForces (+ (Variables|CartMovement|GetRedAndBlueForces) (Variables|CartMovement|GetPlayerCartForce))))
            (Variables|CartMovement|SetBluePlayerIsAtCart false)
            (CallFunction|UpdateCartDirection _output_get_2)
            (goto _label)
            (else
              ;;;[1 1 1] Else if Minion, increment minion count, if >3 move cart
              (if (and (Actor|ActorHasTag (stale _asminion_test) "MinionRed") (Variables|GameManager|GetRedCanPush)) :!label _label_2
                ;;;;[1 0 0] Red
                (bind _output_get_3 (Variables|CartMovement|SetRedAndBlueForces (- (Variables|CartMovement|GetRedAndBlueForces) (Variables|CartMovement|GetMinionCartForce))))
                (CallFunction|UpdateCartDirection _output_get_3)
                ;;;[1 1 1] Set Cart Speed with Direction
                (Variables|CartProgress|SetCartSpeed (* (Variables|CartProgress|GetCurCartVelocity) (Variables|CartProgress|GetCartDirection)) :!label _label_3)
                (elif (and (Actor|ActorHasTag (stale _asminion_test) "MinionBlue") (Variables|GameManager|GetBlueCanPush))
                  ;;;;[0 0 1] Blue
                  (bind _output_get_4 (Variables|CartMovement|SetRedAndBlueForces (+ (Variables|CartMovement|GetRedAndBlueForces) (Variables|CartMovement|GetMinionCartForce))))
                  (CallFunction|UpdateCartDirection _output_get_4)
                  (goto _label_3))))))))
    (:CastFailed
      (bind _asminion_test (Utilities|Casting|CastToMinionTest OtherActor))
      (goto _label_2))))

(event Custom|TickUpdateCart
  (params (delta%20Sec :type Float%20%28single-precision%29))
  (bind _splinepath (Variables|Default|GetSplinePath))
  (bind _cartanimspline (Variables|/Game/Blueprint/CartSpline_BP.CartSpline_BP_C|GetCartAnimSpline _splinepath))
  (bind _output_get (Variables|GameManager|SetGameTimer (- (Variables|GameManager|GetGameTimer) delta%20Sec)))
  (if (<= _output_get 0.0)
    (Variables|Default|SetTimerDidRunOut true)
    (Variables|GameManager|SetGameIsOver true)
    (elif (and (not (Variables|GameManager|GetRedDidWin)) (not (Variables|GameManager|GetBlueDidWin)))
      ;[1 1 1] Move Cart along spline
      (Transformation|SetWorldLocationAndRotation (Variables|Default|GetCartTemp) (Spline|GetLocationatDistanceAlongSpline _cartanimspline (Variables|CartProgress|GetSplineDistance) "World") (Spline|GetRotationatDistanceAlongSpline _cartanimspline (Variables|CartProgress|GetSplineDistance) "World") false false)
      (bind _output_get_2 (Variables|CartProgress|SetSplineDistance (Math|Float|Clamp(Float) (+ (Variables|CartProgress|GetSplineDistance) (Variables|CartProgress|GetCartSpeed)) 0.0 4.8e+04)))
      ;[1 1 1] Convert Distance to Progress Percentage
      (bind _percentage (CallFunction|SplineDistancetoProgressPercentage _output_get_2))
      (CallFunction|CheckCartProgressforAction))))

(event EventBeginPlay
  ;[1 1 1] Get Reference to Spline
  (bind _outactors (Actor|GetAllActorsOfClass "/Game/Blueprint/CartSpline_BP.CartSpline_BP_C"))
  (Variables|Default|SetSplinePath (Utilities|Array|Get(acopy) _outactors))
  ;[1 1 1] Init cart to center of track, not moving
  (bind _distance (CallFunction|ProgressPercentagetoSplineDistance 0.0))
  (Variables|CartProgress|SetSplineDistance _distance)
  (Variables|CartProgress|SetCartSpeed 0.0)
  ;[1 1 1] TMP
  (Input|EnableInput (Game|GetPlayerController 0))
  ;[1 1 1] Set Player Tag: MOVE to Player blueprint or GM class?
  (bind _outactors_2 (Actor|GetAllActorsOfClass "/Game/ThirdPersonBP/Blueprints/ThirdPersonCharacter.ThirdPersonCharacter_C"))
  (Variables|/Script/Engine.Actor|SetTags (Utilities|Array|Get(acopy) _outactors_2) (Utilities|Array|MakeArray "PlayerRed"))
  ;[1 1 1] Get Reference to change weather
  (bind _outactors_3 (Actor|GetAllActorsOfClass "/Game/ShaderTests/BP_GlobalClimate.BP_GlobalClimate_C"))
  (Variables|Default|SetGlobalClimate (Utilities|Array|Get(acopy) _outactors_3))
  ;[1 1 1] Init game timer for checkpoint limit
  (Variables|GameManager|SetGameTimer (Variables|GameManager|GetTimeLimitToCheckpoint)))

(event Input|KeyboardEvents|T
  (params (Key :type Key%20Structure :default "AnyKey"))
  ;[1 1 1] TMP: FlipCartDirection
  (:Pressed
    ;[1 1 1] TMP: hit T to swap to blue team, test cart directions
    (bind _outactors (Actor|GetAllActorsOfClass "/Game/ThirdPersonBP/Blueprints/ThirdPersonCharacter.ThirdPersonCharacter_C"))
    (Variables|/Script/Engine.Actor|SetTags (Utilities|Array|Get(acopy) _outactors) (Utilities|Array|MakeArray "PlayerBlue"))))

(fn ConstructionScript)

(fn GetCartProgress
  (return (Variables|CartProgress|GetCartProgressPercentage)))

(fn InitCartatProgress
  (params (progress :type Float%20%28single-precision%29))
  (bind _splinepath (Variables|Default|GetSplinePath))
  (bind _cartanimspline (Variables|/Game/Blueprint/CartSpline_BP.CartSpline_BP_C|GetCartAnimSpline _splinepath))
  (Variables|CartProgress|SetSplineDistance 0.0)
  ;[1 1 1] Move Cart along spline
  (Transformation|SetWorldLocationAndRotation (Variables|Default|GetCartTemp) (Spline|GetLocationatDistanceAlongSpline _cartanimspline (Variables|CartProgress|GetSplineDistance) "World") (Spline|GetRotationatDistanceAlongSpline _cartanimspline (Variables|CartProgress|GetSplineDistance) "World") false false))

(fn SplineDistancetoProgressPercentage
  (params (distance :type Float%20%28single-precision%29))
  ;[1 1 1] Convert Distance Along Spline to Progress Percentage Base1 = -100; Base2 = 100; StartPoint = 0
  (bind _output_get (Variables|CartProgress|SetCartProgressPercentage (- (* (/ distance 4.8e+04) 2e+02) 1e+02)))
  (return _output_get))

(fn ProgressPercentagetoSplineDistance
  (params (percentage :type Float%20%28single-precision%29))
  ;[1 1 1] Convert Percent of spline traversed [-100,100] to spline distance along track [0,48000]
  (bind _output_get (Variables|CartProgress|SetSplineDistance (* (/ (+ percentage 1e+02) 2e+02) 4.8e+04)))
  (return _output_get))

(fn UpdateCartDirection
  (params (SumForcesOnCart :type Float%20%28single-precision%29))
  (bind _minforcetopush (Variables|CartMovement|GetMinForceToPush))
  (if (Variables|CartMovement|GetRedPlayerIsAtCart)
    ;[1 1 1] If Either player is only player at cart, overpowers all minions and pushes cart
    ;;[1 0 0] Red
    (if (Variables|CartMovement|GetBluePlayerIsAtCart)
      ;[1 1 1] Push Cart in direction of greater force if either team is above minimum requred force
      (if (>= SumForcesOnCart _minforcetopush) :!label _label
        ;;[1 0 0] Red
        (Variables|CartProgress|SetCartDirection 1.0)
        (elif (<= SumForcesOnCart (* _minforcetopush -1.0))
          ;;[0 0 1] Blue
          (Variables|CartProgress|SetCartDirection -1.0)
          (else
            ;;[0 1 0] NoMovement
            (Variables|CartProgress|SetCartDirection 0.0))))
      (else
        (Variables|CartProgress|SetCartDirection 1.0)))
    (else
      ;;[0 0 1] Blue
      (if (Variables|CartMovement|GetBluePlayerIsAtCart)
        (Variables|CartProgress|SetCartDirection -1.0)
        (else
          (goto _label)))))
  (return))

(fn CheckCartProgressforAction
  (if (>= (Variables|CartProgress|GetCartProgressPercentage) 2e+01)
    (if (>= (Variables|CartProgress|GetCartProgressPercentage) 5e+01)
      (if (>= (Variables|CartProgress|GetCartProgressPercentage) 8e+01)
        (if (>= (Variables|CartProgress|GetCartProgressPercentage) 1e+02)
          ;[1 0 0] Red Endpoint
          (Variables|GameManager|SetRedDidWin true)
          (Variables|GameManager|SetGameIsOver true)
          ;[1 1 1] Blow Up Base and end game
          (bind _outactors (Actor|GetAllActorsOfClass "/Game/ShaderTests/BP_BombExplosion.BP_BombExplosion_C"))
          (for _array_element _outactors
            (if (Actor|ActorHasTag _array_element "BaseBlue")
              (bind _asbp_bomb_explosion (Utilities|Casting|CastToBP_BombExplosion _array_element))
              (Default|ExplodeBase _asbp_bomb_explosion)
              (Variables|CartProgress|SetCartSpeed 0.0)))
          (else
            (if (Variables|Default|GetisWinter) :!label _label
              (Variables|Default|SetisWinter false)
              (Variables|CartProgress|SetCurCartVelocity 12.0)
              (Variables|CartProgress|SetCartSpeed (* (Variables|CartProgress|GetCurCartVelocity) (Variables|CartProgress|GetCartDirection)))
              ;[1 1 1] Init Weather Chane at +-50%, change again at +-80%
              (Default|ToggleWeatherSystem (Variables|Default|GetGlobalClimate) :!label _label_2)
              (Development|PrintString "mmmmmmmmmmmmmmmmmmmmmmm"))))
        (else
          (if (not (Variables|Default|GetisWinter)) :!label _label_3
            (Variables|Default|SetisWinter true)
            ;[1 1 1] Slow Cart Down in Snow
            (Variables|CartProgress|SetCurCartVelocity 8.0)
            (Variables|CartProgress|SetCartSpeed (* (Variables|CartProgress|GetCurCartVelocity) (Variables|CartProgress|GetCartDirection)))
            (goto _label_2))))
      (else
        ;[1 0 0] Red Checkpoint
        (if (not (Variables|GameManager|GetTimerIsActive))
          (Variables|GameManager|SetTimerIsActive true)
          (Variables|GameManager|SetBlueCanPush false)
          ;[1 1 1] Start Timer & Linked HUD
          (CallFunction|StartBaseTimer :!label _label_4))))
    (elif (<= (Variables|CartProgress|GetCartProgressPercentage) -2e+01)
      (if (<= (Variables|CartProgress|GetCartProgressPercentage) -5e+01)
        (if (<= (Variables|CartProgress|GetCartProgressPercentage) -8e+01)
          (if (<= (Variables|CartProgress|GetCartProgressPercentage) -1e+02)
            ;[0 0 1] Blue Endpoint
            (Variables|GameManager|SetBlueDidWin true)
            (Variables|GameManager|SetGameIsOver true)
            ;[1 1 1] Blow Up Base and end game
            (bind _outactors_2 (Actor|GetAllActorsOfClass "/Game/ShaderTests/BP_BombExplosion.BP_BombExplosion_C"))
            (for _array_element_2 _outactors_2
              (if (Actor|ActorHasTag _array_element_2 "BaseRed")
                (bind _asbp_bomb_explosion_2 (Utilities|Casting|CastToBP_BombExplosion _array_element_2))
                (Default|ExplodeBase _asbp_bomb_explosion_2)
                (Variables|CartProgress|SetCartSpeed 0.0)))
            (else
              (goto _label)))
          (else
            (goto _label_3)))
        (else
          ;[0 0 1] Blue Checkpoint
          (if (not (Variables|GameManager|GetTimerIsActive))
            (Variables|GameManager|SetTimerIsActive true)
            (Variables|GameManager|SetRedCanPush false)
            (goto _label_4)))))))

(fn GetCartWorldLocation
  (bind _cartprogress (CallFunction|GetCartProgress))
  (bind _distance (CallFunction|ProgressPercentagetoSplineDistance _cartprogress))
  (return (Spline|GetLocationatDistanceAlongSpline (Variables|/Game/Blueprint/CartSpline_BP.CartSpline_BP_C|GetCartAnimSpline (Variables|Default|GetSplinePath)) _distance "World")))

(fn StartBaseTimer
  (Variables|GameManager|SetGameTimer (Variables|GameManager|GetTimeLimitToBase)))